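; LifeSupport is a destructible objective actor whose destruction awards score to the player team and ends the game.
; BeginPlay caches references to the custom game state and game instance.
; AnyDamage subtracts floored damage from Health; at zero or below it adds points to the game instance's PlayerTeamScore, calls EndGame on the game state, destroys itself and plays an explosion sound at the LifeBase location.
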(event EventAnyDamage
  (params (Damage :type Float%20%28single-precision%29) (DamageType :type Damage%20Type%20Object%20Reference) (InstigatedBy :type Controller%20Object%20Reference) (DamageCauser :type Actor%20Object%20Reference))
  (bind _gameinstance (Variables|Default|GetGameInstance))
  ;[1 1 1] Handles taking damage
  (Variables|Default|SetHealth (- (Variables|Default|GetHealth) (Math|Float|Floor Damage)))
  (if (<= (Variables|Default|GetHealth) 0)
    ;[1 1 1] Sets game scoring
    (Variables|/Game/Blueprints/NewGameInstance.NewGameInstance_C|SetPlayerTeamScore _gameinstance (+ (Variables|/Game/Blueprints/NewGameInstance.NewGameInstance_C|GetPlayerTeamScore _gameinstance) 1500))
    (Default|EndGame (Variables|Default|GetGameState))
    (Actor|DestroyActor)
    (Audio|PlaySoundatLocation "/Game/Sounds/Explo3c_Cue.Explo3c_Cue" (Transformation|GetWorldLocation (Variables|Default|GetLifeBase)))))

(event EventBeginPlay
  ;[1 1 1] Create game variables
  (Utilities|FlowControl|Sequence
    (:then_0
      (bind _asnew_game_state (Utilities|Casting|CastToNewGameState (Game|GetGameState)))
      (Variables|Default|SetGameState _asnew_game_state))
    (:then_1
      (bind _asnew_game_instance (Utilities|Casting|CastToNewGameInstance (Game|GetGameInstance)))
      (Variables|Default|SetGameInstance _asnew_game_instance))))

(fn ConstructionScript)