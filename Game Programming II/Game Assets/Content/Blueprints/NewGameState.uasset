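; NewGameState is a game state Blueprint that decides victory or defeat by team score in a starfighter game.
; On BeginPlay it caches the player's BP_Starfighter pawn and the NewGameInstance, which holds both team scores.
; Its EndGame event compares those scores to ScoreGoal, player team first, and sets the Victory or Defeat flag, ignoring its TeamScore input.
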(event Custom|EndGame
  (params (TeamScore :type Integer))
  (bind _gameinstance (Variables|Default|GetGameInstance))
  (bind _scoregoal (Variables|Default|GetScoreGoal))
  ;[1 1 1] Checks to see if the game is over
  (if (>= (Variables|/Game/Blueprints/NewGameInstance.NewGameInstance_C|GetPlayerTeamScore _gameinstance) _scoregoal)
    (Variables|Default|SetVictory true)
    (elif (>= (Variables|/Game/Blueprints/NewGameInstance.NewGameInstance_C|GetEnemyTeamScore _gameinstance) _scoregoal)
      (Variables|Default|SetDefeat true))))

(event EventBeginPlay
  ;[1 1 1] Casts game variables
  (bind _asbp_starfighter (Utilities|Casting|CastToBP_Starfighter (Game|Player|GetPlayerPawn 0)))
  (Variables|Default|SetStarfighter _asbp_starfighter)
  (bind _asnew_game_instance (Utilities|Casting|CastToNewGameInstance (Game|GetGameInstance)))
  (Variables|Default|SetGameInstance _asnew_game_instance))

(fn ConstructionScript)