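; Enemy laser projectile Blueprint that damages the actor it hits and explodes.
; Tick moves it by a Speed-scaled local offset without sweep, then runs a Delay that destroys it and spawns an explosion when its lifetime ends.
; On Hit, it applies fixed damage to the other actor, destroys itself and spawns the explosion at the hit location.
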(event EventTick
  (params (DeltaSeconds :type Float%20%28single-precision%29))
  ;[1 1 1] Handles moving projectiles
  (Transformation|AddActorLocalOffset (* (Variables|Default|GetSpeed) DeltaSeconds) false)
  ;[1 1 1] Handles laser lifetime
  (Utilities|FlowControl|Delay 12.0)
  (Actor|DestroyActor)
  (Effects|SpawnEmitteratLocation "/Game/StarterContent/Particles/P_Explosion.P_Explosion" (Transformation|GetActorLocation)))

(event EventHit
  (params (MyComp :type Primitive%20Component%20Object%20Reference) (Other :type Actor%20Object%20Reference) (OtherComp :type Primitive%20Component%20Object%20Reference) (bSelfMoved :type Boolean) (HitLocation :type Vector :default "0, 0, 0") (HitNormal :type Vector :default "0, 0, 0") (NormalImpulse :type Vector :default "0, 0, 0") (Hit :type Hit%20Result%20Structure%20%28by%20ref%29))
  ;[1 1 1] Handles applying damage to the actor
  (Utilities|Casting|CastToActor Other
    (:then
      (Game|Damage|ApplyDamage Other 25.0 (Game|GetInstigatorController) self))
    (:CastFailed
      _))
  (Actor|DestroyActor)
  (Effects|SpawnEmitteratLocation "/Game/StarterContent/Particles/P_Explosion.P_Explosion" HitLocation))

(fn ConstructionScript)