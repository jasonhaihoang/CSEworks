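; Game controller for a starfighter game that runs the start, death-restart and quit flow, enemy spawning and scoring.
; A gated Tick with a random Delay spawns random enemy classes ahead of the spawn point, with the interval growing to a clamp.
; Player death clears tracked enemies, whose destroyed callbacks trigger camera shake, and re-enters StartGame through a second gate.
; Score events add to player and enemy totals; the construction script applies spawn locations.
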(event Custom|QuitGame
  ;[1 1 1] Handles the start and end of game
  (Utilities|FlowControl|Sequence
    (:then_0
      (Utilities|FlowControl|Gate false) ; enters at Close
    )
    (:then_1
      (Actor|DestroyActor (Variables|Default|Getstarfighter))
      (CallFunction|PlayCameraShake))))

(event Custom|PlayCameraShake
  ;[1 1 1] Camera shake on death
  (Camera|PlayWorldCameraShake 0 (Transformation|GetActorLocation (Variables|Default|GetPlayerShip)) 0.0 5e+02))

(event Custom|PlayerScoreEvent
  (params (Value :type Integer))
  ;[1 1 1] Primitive game scoring
  (CallFunction|ControlPlayerScore Value))

(event Custom|EnemyScoreEvent
  (params (Value :type Integer))
  ;[1 1 1] Primitive game scoring
  (CallFunction|ControlEnemyScore Value))

(event Custom|EnemyDestroyed
  ;[1 1 1] Handles spawning enemies in random location
  (if (Variables|Default|GetbPlayerDead)
    (CallFunction|PlayCameraShake)))

(event Custom|StartGame
  ;[1 1 1] Handles the start and end of game
  (Variables|Default|SetbPlayerDead false)
  (Utilities|FlowControl|Sequence
    (:then_0
      (Variables|Default|SetSpawnInterval 1.0)
      (CallFunction|ResetSpawnEnemies))
    (:then_1
      (Utilities|FlowControl|Gate false) ; enters at Open
    )))

(event Custom|ResetSpawnEnemies
  (bind _maxhorizspawnoffset (Variables|Default|GetMaxHorizSpawnOffset))
  (bind _actorarray (Variables|Default|GetActorArray))
  (bind _enemyspawnpoint (Variables|Default|GetEnemySpawnPoint))
  ;[1 1 1] Handles spawning enemies in random location
  (Utilities|FlowControl|Gate true) ; enters at Open
)

(event Custom|PlayerKilled
  ;[1 1 1] Handles the start and end of game
  (Variables|Default|SetbPlayerDead true)
  (CallFunction|StopSpawningEnemies)
  (Utilities|FlowControl|Gate false
    (:Exit
      (CallFunction|StartGame))))

(event Custom|StopSpawningEnemies
  (bind _spawnedenemies (Variables|Default|GetSpawnedEnemies))
  (bind _maxhorizspawnoffset (Variables|Default|GetMaxHorizSpawnOffset))
  (bind _actorarray (Variables|Default|GetActorArray))
  (bind _enemyspawnpoint (Variables|Default|GetEnemySpawnPoint))
  ;[1 1 1] Handles spawning enemies in random location
  (for _array_element _spawnedenemies
    (Actor|DestroyActor _array_element))
  (Utilities|Array|Clear _spawnedenemies)
  (Utilities|FlowControl|Gate true) ; enters at Close
)

(event EventBeginPlay
  ;[1 1 1] Handles the start and end of game
  (CallFunction|StartGame))

(event EventTick
  (params (DeltaSeconds :type Float%20%28single-precision%29))
  (bind _maxhorizspawnoffset (Variables|Default|GetMaxHorizSpawnOffset))
  (bind _actorarray (Variables|Default|GetActorArray))
  (bind _enemyspawnpoint (Variables|Default|GetEnemySpawnPoint))
  ;[1 1 1] Handles spawning enemies in random location
  (Utilities|FlowControl|Gate true
    (:Exit
      (Utilities|FlowControl|Sequence
        (:then_0
          (Utilities|FlowControl|Delay (Math|Random|RandomFloatinRange (Variables|Default|GetSpawnInterval) (+ (Variables|Default|GetSpawnInterval) 1.0)))
          (bind _returnvalue (Game|SpawnActorfromClass (Utilities|Array|Get(acopy) _actorarray (Math|Random|RandomInteger (Utilities|Array|Length _actorarray))) (Math|Transform|MakeTransform (+ (Transformation|GetWorldLocation _enemyspawnpoint) (Math|Vector|UnrotateVector (Math|Vector|MakeVector 5e+04 (Math|Random|RandomFloatinRange (* _maxhorizspawnoffset -1.0) _maxhorizspawnoffset) 2e+04) (Transformation|GetActorRotation))) (Transformation|GetWorldRotation _enemyspawnpoint) "5.000000,5.000000,5.000000") false 0))
          (Utilities|Array|Add (Variables|Default|GetSpawnedEnemies) _returnvalue)
          (Game|BindEventtoOnDestroyed _returnvalue (delegate Custom|EnemyDestroyed))
          (Variables|Default|SetSpawnInterval (Math|Float|Clamp(Float) (+ (Variables|Default|GetSpawnInterval) 1.3) 0.7 1e+01)))))))

(fn ConstructionScript
  (Transformation|SetRelativeLocation (Variables|Default|GetPlayerSpawnLocation) false)
  (Transformation|SetRelativeLocation (Variables|Default|GetEnemySpawnLocation) false))

(fn ControlPlayerScore
  (params (Val :type Integer))
  (Variables|Default|SetPlayerScore (+ Val (Variables|Default|GetPlayerScore))))

(fn ControlEnemyScore
  (params (Val :type Integer))
  (Variables|Default|SetEnemyScore (+ Val (Variables|Default|GetEnemyScore))))